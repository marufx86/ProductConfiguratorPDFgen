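; BP_ExportTrigger is an unfinished actor for exporting the current product configurator selection.
; DoFullExport finds the first BP_Configurator, then gathers a game-time timestamp and display names of the currently selected object, environment and camera variants.
; The JSON string, file path and success message are disconnected stubs, so nothing is written, and the event graph is empty.
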(event EventBeginPlay)

(event Collision|EventActorBeginOverlap
  (params (OtherActor :type Actor%20Object%20Reference)))

(event EventTick
  (params (DeltaSeconds :type Float%20%28single-precision%29)))

(fn ConstructionScript)

(fn DoFullExport
  (Utilities|FlowControl|Sequence
    (:then_0
      (bind _outactors (Actor|GetAllActorsOfClass "/Game/ProductConfig/Blueprints/BP_Configurator.BP_Configurator_C"))
      (Utilities|IsValid (Utilities|Array|Get(acopy) _outactors)
        (:Is%20Valid
          (bind _asbp_configurator (Utilities|Casting|CastToBP_Configurator (Utilities|Array|Get(acopy) _outactors))
            (:then
              (Variables|Default|SetFoundConfigurator _asbp_configurator)
              (Variables|Default|SetObjectVariantSetsLocal (Variables|Default|GetObjectVariantSets))
              (Variables|Default|SetEnviroVarSetLocal (Variables|Default|GetEnviroVarSet))
              (Variables|Default|SetCameraVarSetLocal (Variables|Default|GetCameraVarSet))
              (Variables|Default|SetTimestampValue (Utilities|String|ToString(Float) (Utilities|Time|GetGameTimeinSeconds)))
              (Utilities|Array|Clear (Variables|Default|GetVariantDisplayStringsArray))
              (for _array_element (Variables|Default|GetObjectVariantSetsLocal)
                (Utilities|Array|Add (Variables|Default|GetVariantDisplayStringsArray) (Utilities|GetDisplayName (Class|VariantSet|GetVariant (.VariantSet (Utilities|Struct|BreakSTRUCT_VarSet _array_element)) (.currentIndex (Utilities|Struct|BreakSTRUCT_VarSet _array_element))))))
              (Variables|Default|SetEnvironmentDisplayString (Utilities|GetDisplayName (Class|VariantSet|GetVariant (.VariantSet (Utilities|Struct|BreakSTRUCT_VarSet (Variables|Default|GetEnviroVarSetLocal))) (.currentIndex (Utilities|Struct|BreakSTRUCT_VarSet (Variables|Default|GetEnviroVarSetLocal))))))
              (Variables|Default|SetCameraDisplayString (Utilities|GetDisplayName (Class|VariantSet|GetVariant (.VariantSet (Utilities|Struct|BreakSTRUCT_VarSet (Variables|Default|GetCameraVarSetLocal))) (.currentIndex (Utilities|Struct|BreakSTRUCT_VarSet (Variables|Default|GetCameraVarSetLocal)))))))
            (:CastFailed
              (Development|PrintString "No configurator found"))))
        (:Is%20Not%20Valid
          (Development|PrintString "No configurator found"))))))