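; BP_ConfigurationExportHelper is an unfinished helper meant to export a product configurator's state to JSON and generate a PDF.
; Its one function casts the input to BP_Configurator, returning an error on failure and doing nothing further on success.
; Disconnected logic gathers selected variant, environment and camera names for an unused configuration struct.
; The success and failure messages are also disconnected, and no actual JSON or PDF export calls are present.
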(event EventBeginPlay)

(event Collision|EventActorBeginOverlap
  (params (OtherActor :type Actor%20Object%20Reference)))

(event EventTick
  (params (DeltaSeconds :type Float%20%28single-precision%29)))

(fn ConstructionScript)

(fn ExportConfigurationandGeneratePDF
  (params (Configurator :type BP%20Configurator%20Class%20Reference))
  (Utilities|Casting|CastToBP_Configurator
    (:CastFailed
      (return false "Failed to cast Configurator to BP_Configurator"))))